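; A jump pad actor that launches any Character that hits it, but only while it is active.
; A hit on the JumpPad component applies LaunchVelocity additively to the character, or prints a debug message when inactive.
; The OpenDoor event, despite its name, uses a FlipFlop to toggle the active flag and recolor the side and rect lights green for active, red for inactive.
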(event OnComponentHit(JumpPad)
  (params (HitComponent :type Primitive%20Component%20Object%20Reference) (OtherActor :type Actor%20Object%20Reference) (OtherComp :type Primitive%20Component%20Object%20Reference) (NormalImpulse :type Vector :default "0, 0, 0") (Hit :type Hit%20Result%20Structure%20%28by%20ref%29))
  (bind _ascharacter (Utilities|Casting|CastToCharacter OtherActor))
  (if (Variables|Default|GetisJumpadActive?)
    (Character|LaunchCharacter _ascharacter (Variables|Default|GetLaunchVelocity) false false)
    (else
      (Development|PrintString "Jumppad isnt active"))))

(event EventOpenDoor
  (Utilities|FlowControl|FlipFlop
    (:A
      (Variables|Default|SetisJumpadActive? true)
      (Rendering|Components|Light|SetLightColor (Variables|Default|GetSideLight) "(R=0.000000,G=1.000000,B=0.201812,A=1.000000)" true)
      (Rendering|Components|Light|SetLightColor (Variables|Default|GetRectLight) "(R=0.000000,G=1.000000,B=0.257460,A=1.000000)" true))
    (:B
      (Variables|Default|SetisJumpadActive? false)
      (Rendering|Components|Light|SetLightColor (Variables|Default|GetSideLight) "(R=1.000000,G=0.004225,B=0.000000,A=1.000000)" true)
      (Rendering|Components|Light|SetLightColor (Variables|Default|GetRectLight) "(R=1.000000,G=0.000000,B=0.000000,A=1.000000)" true))))

(fn ConstructionScript)