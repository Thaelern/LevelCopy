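; Drawbridge actor that alternates between opening and closing each time its OpenDoor event fires.
; A FlipFlop either calls the OpenDrawBridge graph, which rolls the bridge toward NewRotation.X, or plays a second timeline that rolls it back toward StartRotation.X.
; Each timeline update lerps from the current roll rather than a cached start value, so the easing compounds over the timeline curve.
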(event EventOpenDoor
  (Utilities|FlowControl|FlipFlop
    (:A
      (|OpenDrawBridge))
    (:B
      (bind _newtrack_0 (Timeline|Timeline_1 Play)
        (:Update
          (Transformation|SetActorRotation (Math|Rotator|MakeRotator (Math|Float|Lerp (.roll (Transformation|GetActorRotation)) (.x (Variables|Default|GetStartRotation)) _newtrack_0) 0.0 0.0)))))))

(fn ConstructionScript)