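; BP_CP_Mover is a component that moves its owning actor from its starting location toward an offset position.
; BeginPlay stores the start location, and every Tick adds MoveOffSet to it for the target, with no trigger or return trip.
; Speed is travel distance divided by MoveTime, fed into VInterpTo, so movement eases out rather than lasting exactly MoveTime.
; The new location is set without sweeping.
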(event EventBeginPlay
  ;[1 1 1] Sets original location on begin play
  (Variables|Default|SetOriginalLocation (Transformation|GetActorLocation (Components|GetOwner))))

(event EventTick
  (params (DeltaSeconds :type Float%20%28single-precision%29))
  ;[1 1 1] Calculate Current Location
  (bind _output_get (Variables|Default|SetCurrentLocation (Transformation|GetActorLocation (Components|GetOwner))))
  ;[1 1 1] Calculate Target Location
  (bind _output_get_2 (Variables|Default|SetTargetLocation (+ (Variables|Default|GetOriginalLocation) (Variables|Default|GetMoveOffSet))))
  ;[1 1 1] Calculate Speed
  (bind _output_get_3 (Variables|Default|SetSpeed (/ (Math|Vector|Distance(Vector) (Variables|Default|GetOriginalLocation) (Variables|Default|GetTargetLocation)) (Variables|Default|GetMoveTime))))
  (bind _output_get_4 (Variables|Default|SetNewLocation (Math|Interpolation|VInterpTo _output_get _output_get_2 DeltaSeconds _output_get_3)))
  (Transformation|SetActorLocation (Components|GetOwner) _output_get_4 false false))