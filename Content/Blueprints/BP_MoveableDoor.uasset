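; BP_MoveableDoor is a door actor that slides by an offset when the player enters its trigger box.
; It caches its start location on BeginPlay, and the box overlap sets the destination to that location plus OffsetMovement, then plays a timeline.
; Each update lerps from the current location, not the start, toward the destination, so movement compounds rather than following the curve directly.
; The graph has no logic to close it.
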(event OnComponentBeginOverlap(Box)
  (params (OverlappedComponent :type Primitive%20Component%20Object%20Reference) (OtherActor :type Actor%20Object%20Reference) (OtherComp :type Primitive%20Component%20Object%20Reference) (OtherBodyIndex :type Integer) (bFromSweep :type Boolean) (SweepResult :type Hit%20Result%20Structure%20%28by%20ref%29))
  ;[1 1 1] Grabs overlap with player
  (if (== OtherActor (Game|GetPlayerCharacter 0))
    (Variables|Default|SetisPlayerInRange true)
    (if (Variables|Default|GetisPlayerInRange)
      (Variables|Default|SetDestination (+ (Variables|Default|GetStartPos) (Variables|Default|GetOffsetMovement)))
      (bind _timetoopendoor (Timeline|Timeline_0 Play)
        (:Update
          (Transformation|SetActorLocation (Math|Vector|Lerp(Vector) (Transformation|GetActorLocation) (Variables|Default|GetDestination) _timetoopendoor) false false))))))

(event EventBeginPlay
  (Variables|Default|SetStartPos (Transformation|GetActorLocation)))

(fn ConstructionScript)